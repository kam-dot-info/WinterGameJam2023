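; Spline-driven actor that builds a chain of colour-coded, collidable spline meshes along its spline in the construction script.
; It steps along the spline by SectionLength, adding one mesh per step with tangents clamped to that length so segments follow the curve.
; Each segment gets a dynamic material coloured by the Layer selection and writes to custom depth with a shared stencil value.
; The event graph is unused.
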(fn `UserConstructionScript`
  (bind _spline (`self.Spline`))
  (bind _spline_2 (`self.Spline`))
  (for _index (range (+ (`KismetMathLibrary.FTrunc` (/ (`SplineComponent.GetSplineLength` (`self.Spline`)) (`self.SectionLength`))) 1))
    (bind _returnvalue (`AddComponent|NODE_AddSplineMeshComponent-0`))
    (bind _returnvalue_2 (`PrimitiveComponent.CreateDynamicMaterialInstance` _returnvalue 0 "/Game/Materials/M_LayerMaterial.M_LayerMaterial" "None"))
    (`MaterialInstanceDynamic.SetVectorParameterValue` _returnvalue_2 "Colour" (select `int` (`self.Layer`) :`0` (struct :`B` 0.5 :`A` 1.0) :`1` (struct :`G` 0.5 :`A` 1.0) :`2` (struct :`R` 0.5 :`A` 1.0) :!type "LinearColor Structure"))
    (`PrimitiveComponent.SetRenderCustomDepth` _returnvalue true)
    (`PrimitiveComponent.SetCustomDepthStencilValue` _returnvalue 2)
    (`SplineMeshComponent.SetForwardAxis` _returnvalue "X" true)
    (`PrimitiveComponent.SetCollisionEnabled` _returnvalue "QueryAndPhysics")
    (bind _returnvalue_3 (* _index (`self.SectionLength`)))
    (bind _returnvalue_4 (* (+ _index 1) (`self.SectionLength`)))
    (`SplineMeshComponent.SetStartAndEnd` _returnvalue (`SplineComponent.GetLocationAtDistanceAlongSpline` _spline_2 _returnvalue_3 "Local") (`KismetMathLibrary.ClampVectorSize` (`SplineComponent.GetTangentAtDistanceAlongSpline` _spline_2 _returnvalue_3 "Local") 0.0 (`self.SectionLength`)) (`SplineComponent.GetLocationAtDistanceAlongSpline` _spline _returnvalue_4 "Local") (`KismetMathLibrary.ClampVectorSize` (`SplineComponent.GetTangentAtDistanceAlongSpline` _spline _returnvalue_4 "Local") 0.0 (`self.SectionLength`)) true)))