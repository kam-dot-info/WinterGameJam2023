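; Start platform that plays the Robo-Ball intro when play begins, then hands the view to the player.
; BeginPlay hides the pawn, views from the platform and plays a stand-in skeletal animation with a transform sound, in short or long timing per ShortIntro.
; It then swaps in the real ball at the mesh's Base socket, blends the camera to it and enables death.
; Left-click functions only toggle actor tick.
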(event `self.ReceiveBeginPlay`
  (bind _playermesh (`self.PlayerMesh`))
  (bind _playermesh_2 (`self.PlayerMesh`))
  (bind _playermesh_3 (`self.PlayerMesh`))
  (bind _as_robo__ball (`self.As Robo- Ball`))
  (bind _sphere (`/Game/Blueprint/Char/Robo-Ball.Sphere` _as_robo__ball))
  (bind _asrobo__ball (cast `/Game/Blueprint/Char/Robo-Ball` (`GameplayStatics.GetPlayerPawn` 0)))
  (bind _output_get (set `self.As Robo- Ball` _asrobo__ball))
  (`self.SetActorHiddenInGame` _output_get true)
  (bind _sphere_2 (`/Game/Blueprint/Char/Robo-Ball.Sphere` _output_get))
  (`PrimitiveComponent.SetSimulatePhysics` _sphere_2 true)
  (`SceneComponent.SetVisibility` _sphere_2 false false)
  (`PlayerController.SetViewTargetWithBlend` (`GameplayStatics.GetPlayerController` 0) self 0.0 "VTBlend_Linear" 0.0 false)
  (if (`self.ShortIntro?`)
    (`SkeletalMeshComponent.PlayAnimation` _playermesh_2 "/Game/Assets/Robot/Skeleton/Robot-Ball-SK_Anim.Robot-Ball-SK_Anim" false)
    (`SkeletalMeshComponent.SetPosition` _playermesh_2 1.236602 true)
    (`SkeletalMeshComponent.Play` _playermesh_2 false)
    (`KismetSystemLibrary.Delay` 1.05)
    (`GameplayStatics.PlaySound2D` "/Game/Sound/RobotTransform/RobotTransform.RobotTransform" 1.0 1.0 0.0 null null)
    (`KismetSystemLibrary.Delay` 1.463398)
    (else
      (`SkeletalMeshComponent.PlayAnimation` _playermesh_3 "/Game/Assets/Robot/Skeleton/Robot-Ball-SK_Anim.Robot-Ball-SK_Anim" false)
      (`SkeletalMeshComponent.Stop` _playermesh_3)
      (`KismetSystemLibrary.Delay` 1.0)
      (`SkeletalMeshComponent.Play` _playermesh_3 false)
      (`KismetSystemLibrary.Delay` 2.2)
      (`GameplayStatics.PlaySound2D` "/Game/Sound/RobotTransform/RobotTransform.RobotTransform" 1.0 1.0 0.0 null null)
      (`KismetSystemLibrary.Delay` 1.8)))
  (`SceneComponent.SetVisibility` _playermesh false false)
  (`SceneComponent.K2_SetWorldLocation` (`/Game/Blueprint/Char/Robo-Ball.Sphere` (`self.As Robo- Ball`)) (`SceneComponent.GetSocketLocation` _playermesh "Base") false false)
  (`self.SetActorHiddenInGame` _as_robo__ball false)
  (`PrimitiveComponent.SetSimulatePhysics` _sphere true)
  (`SceneComponent.SetVisibility` _sphere true false)
  (`PlayerController.SetViewTargetWithBlend` (`GameplayStatics.GetPlayerController` 0) (`self.As Robo- Ball`) 1.0 "VTBlend_EaseOut" 0.5 false)
  (`/Game/Blueprint/Char/Robo-Ball.EnableDeath` (`self.As Robo- Ball`)))

(fn `LeftClickFunction`
  (`self.SetActorTickEnabled` true))

(fn `LeftClickUnpressedFunction`
  (`self.SetActorTickEnabled` false))

(fn `UserConstructionScript`)