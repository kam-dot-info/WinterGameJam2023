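; End-of-level platform that plays a robot kiss cutscene when the Robo-Ball enters its trigger box.
; On overlap it makes the ball unkillable, disables its physics and blends the view to the platform's camera.
; A timeline pulls the ball onto the mesh socket, moves the spring arm and tilts both robots, with events swapping in animated meshes and firing hearts and sound.
; When it finishes, it shows the end screen with the next level name.
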(event `self.ReceiveBeginPlay`
  (bind _playermesh2 (`self.PlayerMesh2`))
  (`SkeletalMeshComponent.PlayAnimation` _playermesh2 "/Game/Assets/Robot/Skeleton/RobotEndingAnimation.RobotEndingAnimation" false)
  (`SkeletalMeshComponent.Stop` _playermesh2))

(event `self.Box.OnComponentBeginOverlap`
  (params (OverlappedComponent :type "PrimitiveComponent Object Reference") (OtherActor :type "Actor Object Reference") (OtherComp :type "PrimitiveComponent Object Reference") (OtherBodyIndex :type Integer) (bFromSweep :type Boolean) (SweepResult :type "HitResult Structure (by ref)"))
  (bind (_playertransform_location _playertransform_rotation) (`KismetMathLibrary.BreakTransform` (`self.PlayerTransform`)))
  (bind _playermesh (`self.PlayerMesh`))
  (bind _as_robo__ball (`self.As Robo- Ball`))
  (bind _ingameui (`/Game/Blueprint/Char/Robo-Ball.IngameUI` (`self.As Robo- Ball`)))
  (bind _asrobo__ball (cast `/Game/Blueprint/Char/Robo-Ball` OtherActor))
  (bind _output_get (set `self.As Robo- Ball` _asrobo__ball))
  (set `/Game/Blueprint/Char/Robo-Ball.CanDie?` false _output_get)
  (`/Game/Blueprint/Char/Robo-Ball.ReachedTheEnd` _output_get)
  (`PrimitiveComponent.SetSimulatePhysics` (`/Game/Blueprint/Char/Robo-Ball.Sphere` _output_get) false)
  (`PlayerController.SetViewTargetWithBlend` (`GameplayStatics.GetPlayerController` 0) self 2.0 "VTBlend_EaseInOut" 1.0 false)
  (`UserWidget.PlayAnimationReverse` _ingameui (`/Game/Blueprint/UI/InGameUI.Fade` _ingameui) 1.0 false)
  (set `self.PlayerTransform` (`SceneComponent.K2_GetComponentToWorld` (`/Game/Blueprint/Char/Robo-Ball.Sphere` (`self.As Robo- Ball`))))
  (bind (_direction _cameraheight _robotkiss _charlerp) (`Timeline|Timeline` :!via `PlayFromStart`)
    (:`Update`
      (`SceneComponent.K2_SetWorldLocationAndRotation` (`/Game/Blueprint/Char/Robo-Ball.Sphere` (`self.As Robo- Ball`)) (`KismetMathLibrary.VLerp` _playertransform_location (`SceneComponent.GetSocketLocation` (`self.PlayerMesh`) "Base") _charlerp) (`KismetMathLibrary.RLerp` _playertransform_rotation (struct) _charlerp) false false)
      (`SceneComponent.K2_SetRelativeLocationAndRotation` (`self.SpringArm`) (`KismetMathLibrary.VLerp` (0.0 40.0 80.0) (-400.0 40.0 340.0) _cameraheight) (struct :`Pitch` -5.0) false false)
      (bind _returnvalue (`KismetMathLibrary.Lerp` 0.0 13.0 _robotkiss))
      (`SceneComponent.K2_SetRelativeRotation` (`self.PlayerMesh`) (`KismetMathLibrary.MakeRotator` _returnvalue) false false)
      (`SceneComponent.K2_SetRelativeRotation` (`self.PlayerMesh2`) (`KismetMathLibrary.MakeRotator` _returnvalue 0.0 180.0) false false))
    (:`Finished`
      (bind _returnvalue_2 (`|CreateWidget` "/Game/Blueprint/UI/EndScreen.EndScreen_C"))
      (`UserWidget.AddToViewport` _returnvalue_2 0)
      (set `/Game/Blueprint/UI/EndScreen.NextLevelName` (`self.NextLevelName`) _returnvalue_2))
    (:`PlayerTransformend`
      (`self.SetActorHiddenInGame` _as_robo__ball true)
      (`SceneComponent.SetVisibility` (`/Game/Blueprint/Char/Robo-Ball.Sphere` _as_robo__ball) false false)
      (`SceneComponent.SetHiddenInGame` _playermesh false false)
      (`SkeletalMeshComponent.PlayAnimation` _playermesh "/Game/Assets/Robot/Skeleton/RobotEndingAnimation.RobotEndingAnimation" false)
      (`SkeletalMeshComponent.PlayAnimation` (`self.PlayerMesh2`) "/Game/Assets/Robot/Skeleton/RobotEndingAnimation.RobotEndingAnimation" false))
    (:`StartHearts`
      (`ActorComponent.Activate` (`self.LoveHearts2`) false)
      (`ActorComponent.Activate` (`self.LoveHearts1`) false)
      (`ActorComponent.Activate` (`self.LoveHearts`) false)
      (`GameplayStatics.PlaySound2D` "/Game/Sound/RobotKiss/RobotKiss.RobotKiss" 1.0 1.0 0.0 null null))))

(fn `UserConstructionScript`)