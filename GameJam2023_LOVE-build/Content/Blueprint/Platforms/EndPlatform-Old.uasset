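; End platform Blueprint that plays the level-finish cinematic when the Robo-Ball rolls into its trigger box.
; It hides the ball, stops its physics and death, notifies it of reaching the end, then blends the camera to itself.
; After a delay, a timeline raises the spring-arm camera, drives Legs/Arms/Body morph targets on two robot meshes and tilts them into a kiss, with the second mesh's animation played in reverse.
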(event `self.Box.OnComponentBeginOverlap`
  (params (OverlappedComponent :type "PrimitiveComponent Object Reference") (OtherActor :type "Actor Object Reference") (OtherComp :type "PrimitiveComponent Object Reference") (OtherBodyIndex :type Integer) (bFromSweep :type Boolean) (SweepResult :type "HitResult Structure (by ref)"))
  (bind _playermesh2 (`self.PlayerMesh2`))
  (bind _playermesh (`self.PlayerMesh`))
  (bind _asrobo__ball (cast `/Game/Blueprint/Char/Robo-Ball` OtherActor))
  (bind _output_get (set `self.As Robo- Ball` _asrobo__ball))
  (`self.SetActorHiddenInGame` _output_get true)
  (bind _sphere (`/Game/Blueprint/Char/Robo-Ball.Sphere` _output_get))
  (`PrimitiveComponent.SetSimulatePhysics` _sphere false)
  (`SceneComponent.SetVisibility` _sphere false false)
  (set `/Game/Blueprint/Char/Robo-Ball.CanDie?` false _output_get)
  (`/Game/Blueprint/Char/Robo-Ball.ReachedTheEnd` _output_get)
  (`PlayerController.SetViewTargetWithBlend` (`GameplayStatics.GetPlayerController` 0) self 2.0 "VTBlend_EaseInOut" 1.0 false)
  (`SceneComponent.SetHiddenInGame` (`self.PlayerMesh`) false false)
  (`KismetSystemLibrary.Delay` 2.0)
  (`SkeletalMeshComponent.SetPlayRate` _playermesh2 -1.0)
  (`SkeletalMeshComponent.Play` _playermesh2 false)
  (bind (_direction _cameraheight _body _arms _legs _robotkiss) (`Timeline|RobotExpandTimeline` :!via `PlayFromStart`)
    (:`Update`
      (`SceneComponent.K2_SetRelativeLocationAndRotation` (`self.SpringArm`) (`KismetMathLibrary.VLerp` (0.0 40.0 80.0) (-400.0 40.0 340.0) _cameraheight) (struct :`Pitch` -5.0) false false)
      (`SkeletalMeshComponent.SetMorphTarget` _playermesh "Legs" _legs true)
      (`SkeletalMeshComponent.SetMorphTarget` (`self.PlayerMesh2`) "Legs" _legs true)
      (`SkeletalMeshComponent.SetMorphTarget` _playermesh "Arms" _arms true)
      (`SkeletalMeshComponent.SetMorphTarget` (`self.PlayerMesh2`) "Arms" _arms true)
      (`SkeletalMeshComponent.SetMorphTarget` _playermesh "Body" _body true)
      (`SkeletalMeshComponent.SetMorphTarget` (`self.PlayerMesh2`) "Body" _body true)
      (bind _returnvalue (`KismetMathLibrary.Lerp` 0.0 13.0 _robotkiss))
      (`SceneComponent.K2_SetRelativeRotation` (`self.PlayerMesh`) (`KismetMathLibrary.MakeRotator` _returnvalue) false false)
      (`SceneComponent.K2_SetRelativeRotation` (`self.PlayerMesh2`) (`KismetMathLibrary.MakeRotator` _returnvalue 0.0 180.0) false false))))

(event `self.ReceiveBeginPlay`
  (bind _playermesh (`self.PlayerMesh`))
  (`SkeletalMeshComponent.SetMorphTarget` _playermesh "Legs" 1.0 true)
  (`SkeletalMeshComponent.SetMorphTarget` (`self.PlayerMesh2`) "Legs" 1.0 true)
  (`SkeletalMeshComponent.SetMorphTarget` _playermesh "Arms" 1.0 true)
  (`SkeletalMeshComponent.SetMorphTarget` (`self.PlayerMesh2`) "Arms" 1.0 true)
  (`SkeletalMeshComponent.SetMorphTarget` _playermesh "Body" 1.0 true)
  (`SkeletalMeshComponent.SetMorphTarget` (`self.PlayerMesh2`) "Body" 1.0 true))

(fn `UserConstructionScript`)