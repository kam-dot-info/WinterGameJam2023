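; Click-driven depth platform that slides along world X between depth positions, with its colour shifting to match.
; Left click plays and right click reverses a timeline that drives location and a shared dynamic material colour, with a DoOnce-gated stop event able to halt forward travel.
; StartingDepth seeds the timeline's playback position.
; The construction script fits the middle and edge cubes to WallScale and rotates the direction arrow and face widget.
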(event `LeftClickMovement`
  (bind (_returnvalue_x _returnvalue_y _returnvalue_z) (`KismetMathLibrary.BreakVector` (`self.K2_GetActorLocation`)))
  (bind _mi_layercolour (`self.MI_LayerColour`))
  (`GameplayStatics.PlaySound2D` "/Game/Sound/CubeMovement/CubeMovement.CubeMovement" 1.0 1.0 0.0 null null)
  (bind (_direction _depth _depthcolour) (`Timeline|PlatformMovement` :!label _label)
    (:`Update`
      (`self.K2_SetActorLocation` (`KismetMathLibrary.MakeVector` (`KismetMathLibrary.Lerp` 0.0 256.0 _depth) _returnvalue_y _returnvalue_z))
      (`/Engine/EditorBlueprintResources/StandardMacros.IsValid` _mi_layercolour
        (:`Is Valid`
          (`MaterialInstanceDynamic.SetVectorParameterValue` _mi_layercolour "Colour" _depthcolour))))
    (:`StopEvent`
      (`/Engine/EditorBlueprintResources/StandardMacros.DoOnce` (== (`self.StartingDepth`) 1) :!label _label_2
        (:`Completed`
          (`TimelineComponent.Stop` (`self.PlatformMovement`)))))
    (:`ResetStop`
      (goto _label_2 :!via `Reset`))))

(event `RightClickMovement`
  (`GameplayStatics.PlaySound2D` "/Game/Sound/CubeMovement/CubeMovement.CubeMovement" 1.0 1.0 0.0 null null)
  (goto _label :!via `Reverse`))

(event `self.ReceiveBeginPlay`
  (bind _returnvalue (`PrimitiveComponent.CreateDynamicMaterialInstance` (`self.MiddleCube`) 0 "/Game/Materials/M_LayerMaterial.M_LayerMaterial" "None"))
  (set `self.MI_LayerColour` _returnvalue)
  (`TimelineComponent.SetPlaybackPosition` (`self.PlatformMovement`) (select `int` (`self.StartingDepth`) :`0` 0.0 :`1` 0.25 :`2` 0.5 :!type "Float (single-precision)") false true)
  (`PrimitiveComponent.SetMaterial` (`self.Cube1`) 0 (`self.MI_LayerColour`))
  (`PrimitiveComponent.SetMaterial` (`self.Cube2`) 0 (`self.MI_LayerColour`))
  (`PrimitiveComponent.SetMaterial` (`self.Cube3`) 0 (`self.MI_LayerColour`))
  (`PrimitiveComponent.SetMaterial` (`self.Cube4`) 0 (`self.MI_LayerColour`)))

(fn `LeftClickFunction`
  (`self.LeftClickMovement`))

(fn `RightClickFunction`
  (`self.RightClickMovement`))

(fn `UserConstructionScript`
  (bind (_wallscale_x _wallscale_y _wallscale_z) (`KismetMathLibrary.BreakVector` (`self.WallScale`)))
  (`TimelineComponent.SetPlaybackPosition` (`self.PlatformMovement`) (select `int` (`self.StartingDepth`) :`0` 0.0 :`1` 0.25 :`2` 0.5 :!type "Float (single-precision)") false true)
  (`SceneComponent.K2_SetRelativeLocation` (`self.TopEdgeCubes`) (`KismetMathLibrary.MakeVector` 0.0 0.0 (* _wallscale_z 50.0)) false false)
  (`SceneComponent.K2_SetRelativeLocation` (`self.BottomEdgeCubss`) (`KismetMathLibrary.MakeVector` 0.0 0.0 (* (* -1.0 _wallscale_z) 50.0)) false false)
  (`SceneComponent.SetRelativeScale3D` (`self.MiddleCube`) (`self.WallScale`))
  (`SceneComponent.K2_SetRelativeRotation` (`self.DirectionArrow`) (`KismetMathLibrary.MakeRotator` 90.0 (`self.DirectionArrowRotation`)) false false)
  (`SceneComponent.K2_SetRelativeRotation` (`self.FaceWidget`) (`KismetMathLibrary.MakeRotator` (`self.DirectionArrowRotation`) 0.0 90.0) false false)
  (`SceneComponent.K2_SetRelativeRotation` (`self.FaceWidget`) (`KismetMathLibrary.MakeRotator` (`self.DirectionArrowRotation`) 0.0 90.0) false false))