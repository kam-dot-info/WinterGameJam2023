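; Sliding platform that the player drags along a spline with the mouse cursor.
; Clicking the actor toggles Tick, and left-click press/release functions enable or disable it; each tick snaps the SpringArm to the spline point nearest the cursor's trace hit.
; BeginPlay tints the cubes through a shared dynamic material coloured by StartingDepth.
; The construction script fits middle and edge cubes to WallScale and rotates the direction arrow.
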(event `self.ReceiveActorOnClicked`
  (params (ButtonPressed :type "Key Structure"))
  (bind _isa (`/Engine/EditorBlueprintResources/StandardMacros.FlipFlop`)
    (:`A`
      _)
    (:`B`
      _))
  (`self.SetActorTickEnabled` _isa))

(event `self.ReceiveTick`
  (params (DeltaSeconds :type "Float (single-precision)"))
  (`SceneComponent.K2_SetWorldLocation` (`self.SpringArm`) (`SplineComponent.FindLocationClosestToWorldLocation` (`self.Spline`) (`.Location` (`GameplayStatics.BreakHitResult` (`PlayerController.GetHitResultUnderCursorByChannel` (`GameplayStatics.GetPlayerController` 0) "TraceTypeQuery1" true))) "World") false false))

(event `self.ReceiveBeginPlay`
  (bind _returnvalue (`PrimitiveComponent.CreateDynamicMaterialInstance` (`self.MiddleCube`) 0 "/Game/Materials/M_LayerMaterial.M_LayerMaterial" "None"))
  (set `self.MI_LayerColour` _returnvalue)
  (`PrimitiveComponent.SetMaterial` (`self.Cube1`) 0 (`self.MI_LayerColour`))
  (`PrimitiveComponent.SetMaterial` (`self.Cube2`) 0 (`self.MI_LayerColour`))
  (`PrimitiveComponent.SetMaterial` (`self.Cube3`) 0 (`self.MI_LayerColour`))
  (`PrimitiveComponent.SetMaterial` (`self.Cube4`) 0 (`self.MI_LayerColour`))
  (`MaterialInstanceDynamic.SetVectorParameterValue` (`self.MI_LayerColour`) "Colour" (select `int` (`self.StartingDepth`) :`0` (struct :`B` 0.5 :`A` 1.0) :`1` (struct :`G` 0.5 :`A` 1.0) :`2` (struct :`R` 0.5 :`A` 1.0) :!type "LinearColor Structure")))

(fn `LeftClickFunction`
  (`self.SetActorTickEnabled` true))

(fn `LeftClickUnpressedFunction`
  (`self.SetActorTickEnabled` false))

(fn `UserConstructionScript`
  (bind (_wallscale_x _wallscale_y _wallscale_z) (`KismetMathLibrary.BreakVector` (`self.WallScale`)))
  (`SceneComponent.K2_SetRelativeLocation` (`self.TopEdgeCubes`) (`KismetMathLibrary.MakeVector` 0.0 0.0 (* _wallscale_z 50.0)) false false)
  (`SceneComponent.K2_SetRelativeLocation` (`self.BottomEdgeCubss`) (`KismetMathLibrary.MakeVector` 0.0 0.0 (* (* -1.0 _wallscale_z) 50.0)) false false)
  (`SceneComponent.SetRelativeScale3D` (`self.MiddleCube`) (`self.WallScale`))
  (`SceneComponent.K2_SetRelativeRotation` (`self.DirectionArrow`) (`KismetMathLibrary.MakeRotator` 90.0 (`self.DirectionArrowRotation`)) false false))