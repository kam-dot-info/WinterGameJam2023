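; Start platform actor that plays the robot ball player's intro and then releases the ball.
; On BeginPlay it hides the Robo-Ball pawn, then after a short delay a timeline drives legs, arms and body morph targets on a stand-in PlayerMesh.
; When it finishes, the stand-in hides, the ball reappears with death enabled, and a second timeline tilts the platform.
; Left-click functions only toggle actor tick.
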(event `self.ReceiveBeginPlay`
  (bind _as_robo__ball (`self.As Robo- Ball`))
  (bind _playermesh (`self.PlayerMesh`))
  (bind _sphere (`/Game/Blueprint/Char/Robo-Ball.Sphere` _as_robo__ball))
  (bind _asrobo__ball (cast `/Game/Blueprint/Char/Robo-Ball` (`GameplayStatics.GetPlayerPawn` 0)))
  (bind _output_get (set `self.As Robo- Ball` _asrobo__ball))
  (`self.SetActorHiddenInGame` _output_get true)
  (bind _sphere_2 (`/Game/Blueprint/Char/Robo-Ball.Sphere` _output_get))
  (`PrimitiveComponent.SetSimulatePhysics` _sphere_2 true)
  (`SceneComponent.SetVisibility` _sphere_2 false false)
  (`KismetSystemLibrary.Delay` 1.0)
  (bind (_direction _arms _legs _body) (`Timeline|IntroTimeline` :!via `PlayFromStart`)
    (:`Update`
      (`SkeletalMeshComponent.SetMorphTarget` _playermesh "Legs" _legs true)
      (`SkeletalMeshComponent.SetMorphTarget` _playermesh "Arms" _arms true)
      (`SkeletalMeshComponent.SetMorphTarget` _playermesh "Body" _body true))
    (:`Finished`
      (`SceneComponent.SetVisibility` (`self.PlayerMesh`) false false)
      (`self.SetActorHiddenInGame` _as_robo__ball false)
      (`PrimitiveComponent.SetSimulatePhysics` _sphere true)
      (`SceneComponent.SetVisibility` _sphere true false)
      (`/Game/Blueprint/Char/Robo-Ball.EnableDeath` (`self.As Robo- Ball`))
      (bind (_direction_2 _platformrotation) (`Timeline|Platformrotationtimeline` :!via `PlayFromStart`)
        (:`Update`
          (`SceneComponent.K2_SetRelativeRotation` (`self.StaticMesh`) (`KismetMathLibrary.MakeRotator` 0.0 (`KismetMathLibrary.Lerp` 0.0 -20.0 _platformrotation) 90.0) false false))))))

(fn `LeftClickFunction`
  (`self.SetActorTickEnabled` true))

(fn `LeftClickUnpressedFunction`
  (`self.SetActorTickEnabled` false))

(fn `UserConstructionScript`)